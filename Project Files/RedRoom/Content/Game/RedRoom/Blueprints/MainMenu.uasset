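; RedRoom main menu actor that runs a timed intro with a spotlight, a plane and menu text.
; On BeginPlay it zeroes the spotlight, then after a delay drives two staggered material fades on the plane through a dynamic instance and timelines.
; A parallel, longer delay calls FadeText on the RedRoom_MainMenu widget.
; A separate MusicTrigger event animates the spotlight's intensity with its own timeline.
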(event Custom|MusicTrigger
  (bind _newtrack_0 (Timeline|Timeline_0 Play)
    (:Update
      (Rendering|Components|Light|SetIntensity (Variables|Default|GetSpotLight) _newtrack_0))))

(event EventBeginPlay
  (bind _plane (Variables|Default|GetPlane))
  (Utilities|FlowControl|Sequence
    (:then_0
      (Rendering|Components|Light|SetIntensity (Variables|Default|GetSpotLight) 0.0)
      (Utilities|FlowControl|Delay 19.0)
      (bind _returnvalue (Rendering|Material|CreateDynamicMaterialInstance _plane 0 (Rendering|Material|GetMaterial _plane 0) :!class /Script/Engine.PrimitiveComponent))
      (Rendering|Material|SetMaterial _plane 0 _returnvalue)
      (bind _newtrack_1 (Timeline|Timeline_1 Play)
        (:Update
          (Rendering|Material|SetScalarParameterValue _returnvalue "Fade" _newtrack_1 :!class /Script/Engine.MaterialInstanceDynamic)
          (Utilities|FlowControl|Delay 5.0)
          (bind _newtrack_1_2 (Timeline|Timeline_2 Play)
            (:Update
              (Rendering|Material|SetScalarParameterValue _returnvalue "Fade_1" _newtrack_1_2 :!class /Script/Engine.MaterialInstanceDynamic))))))
    (:then_1
      (Utilities|FlowControl|Delay 27.0)
      (bind _foundwidgets (Widget|GetAllWidgetsOfClass "/Game/Game/RedRoom/UMG/RedRoom_MainMenu.RedRoom_MainMenu_C" false))
      (Default|FadeText (Utilities|Array|Get(acopy) _foundwidgets)))))

(fn ConstructionScript)